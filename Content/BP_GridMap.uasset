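; Grid map actor for a chess-style battle that spawns the starting sword pawns for two teams.
; Shortly after BeginPlay it calls SpawnTeam1 and SpawnTeam2, placing three pawns each at hardcoded grid nodes at opposite ends.
; Each pawn's ChessMovement receives its current node, and second-team pawns spawn rotated and get their team set explicitly.
; An unconnected debug branch finds a path between two nodes and draws spheres along it.
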(event `self.ReceiveBeginPlay`
  (bind _returnvalue (`self.GetNode` (make `GridVector` 1)))
  (bind _returnvalue_2 (`self.GetNode` (make `GridVector` 0)))
  (bind _returnvalue_3 (`self.GetNode` (make `GridVector` 2)))
  (bind _returnvalue_4 (`self.GetNode` (make `GridVector` 9 11)))
  (bind _returnvalue_5 (`self.GetNode` (make `GridVector` 8 11)))
  (bind _returnvalue_6 (`self.GetNode` (make `GridVector` 7 11)))
  (`KismetSystemLibrary.Delay` 0.2)
  (`|ExecutionSequence`
    (:`then_0`
      (`|ExecutionSequence`
        (:`then_0`
          (bind _returnvalue_7 (`|SpawnActorFromClass` "/Game/BP_ChessPawn_Sword.BP_ChessPawn_Sword_C" (`KismetMathLibrary.MakeTransform` (`GridNode.Location` _returnvalue_2)) "AlwaysSpawn" "OverrideRootScale" null null))
          (`ChessMovementComponent.SetNowNode` (`/Game/BP_ChessPawn.ChessMovement` _returnvalue_7) _returnvalue_2))
        (:`then_1`
          (bind _returnvalue_8 (`|SpawnActorFromClass` "/Game/BP_ChessPawn_Sword.BP_ChessPawn_Sword_C" (`KismetMathLibrary.MakeTransform` (`GridNode.Location` _returnvalue)) "AlwaysSpawn" "OverrideRootScale" null null))
          (`ChessMovementComponent.SetNowNode` (`/Game/BP_ChessPawn.ChessMovement` _returnvalue_8) _returnvalue))
        (:`then_2`
          (bind _returnvalue_9 (`|SpawnActorFromClass` "/Game/BP_ChessPawn_Sword.BP_ChessPawn_Sword_C" (`KismetMathLibrary.MakeTransform` (`GridNode.Location` _returnvalue_3)) "AlwaysSpawn" "OverrideRootScale" null null))
          (`ChessMovementComponent.SetNowNode` (`/Game/BP_ChessPawn.ChessMovement` _returnvalue_9) _returnvalue_3))))
    (:`then_1`
      (`|ExecutionSequence`
        (:`then_0`
          (bind _returnvalue_10 (`|SpawnActorFromClass` "/Game/BP_ChessPawn_Sword.BP_ChessPawn_Sword_C" (`KismetMathLibrary.MakeTransform` (`GridNode.Location` _returnvalue_4) (struct :`Yaw` 180.0)) "AlwaysSpawn" "OverrideRootScale" null null))
          (`ChessMovementComponent.SetNowNode` (`/Game/BP_ChessPawn.ChessMovement` _returnvalue_10) _returnvalue_4)
          (`/Game/BP_ChessPawn.SetTeam` _returnvalue_10 1))
        (:`then_1`
          (bind _returnvalue_11 (`|SpawnActorFromClass` "/Game/BP_ChessPawn_Sword.BP_ChessPawn_Sword_C" (`KismetMathLibrary.MakeTransform` (`GridNode.Location` _returnvalue_5) (struct :`Yaw` 180.0)) "AlwaysSpawn" "OverrideRootScale" null null))
          (`ChessMovementComponent.SetNowNode` (`/Game/BP_ChessPawn.ChessMovement` _returnvalue_11) _returnvalue_5)
          (`/Game/BP_ChessPawn.SetTeam` _returnvalue_11 1))
        (:`then_2`
          (bind _returnvalue_12 (`|SpawnActorFromClass` "/Game/BP_ChessPawn_Sword.BP_ChessPawn_Sword_C" (`KismetMathLibrary.MakeTransform` (`GridNode.Location` _returnvalue_6) (struct :`Yaw` 180.0)) "AlwaysSpawn" "OverrideRootScale" null null))
          (`ChessMovementComponent.SetNowNode` (`/Game/BP_ChessPawn.ChessMovement` _returnvalue_12) _returnvalue_6)
          (`/Game/BP_ChessPawn.SetTeam` _returnvalue_12 1))))))

(fn `UserConstructionScript`)