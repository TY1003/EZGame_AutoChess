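; BP_ChessPawn is a chess unit with health, a team, attack animations and a widget-based HP display.
; BeginPlay binds the BP_HP widget to the pawn, and incoming damage lowers Health, destroying the actor at zero.
; DoAttack cycles through attack montages on the skeletal mesh, while DoDamage applies fixed damage to NowTarget.
; SetTeam stores the team index and tints the body material red for one team.
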(event `self.ReceiveBeginPlay`
  (bind _asbp_hp (cast `/Game/UI/BP_HP` (`WidgetComponent.GetUserWidgetObject` (`self.Widget`))))
  (`/Game/UI/BP_HP.InitUI` _asbp_hp self))

(event `self.ReceiveAnyDamage`
  (params (Damage :type "Float (single-precision)") (DamageType :type "DamageType Object Reference") (InstigatedBy :type "Controller Object Reference") (DamageCauser :type "Actor Object Reference"))
  (bind _output_get (set `self.Health` (`KismetMathLibrary.FMax` (- (`self.Health`) Damage))))
  (if (<= _output_get 0.0)
    (`self.K2_DestroyActor`)))

(fn `DoAttack`
  (returns (Return :type "Float (double-precision)"))
  (bind _returnvalue (+ (`self.AttackMontageIndex`) 1))
  (if (> (`KismetArrayLibrary.Array_Length` (`self.AttackMontages`)) 0)
    (bind _returnvalue_2 (`AnimInstance.Montage_Play` (`SkeletalMeshComponent.GetAnimInstance` (`self.SkeletalMesh`)) (`|GetArrayItem` (`self.AttackMontages`) (`self.AttackMontageIndex`)) 1.0 "MontageLength" 0.0 true))
    (set `self.AttackMontageIndex` (`KismetMathLibrary.SelectInt` _returnvalue 0 (< _returnvalue (`KismetArrayLibrary.Array_Length` (`self.AttackMontages`)))))
    (return _returnvalue_2)
    (else
      (return 0.0))))

(fn `DoDamage`
  (`GameplayStatics.ApplyDamage` (`self.NowTarget`) 1.0))

(fn `SetTeam`
  (params (TeamIndex :type Integer))
  (bind _output_get (set `self.TeamIndex` TeamIndex))
  (switch `int` _output_get
    (:`1`
      (`MeshComponent.SetVectorParameterValueOnMaterials` (`self.SkeletalMesh`) "BodyColor" (`KismetMathLibrary.Conv_LinearColorToVector` (struct :`R` 1.0 :`A` 1.0))))))

(fn `UserConstructionScript`)